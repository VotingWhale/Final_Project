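; Cube actor that travels from start to end along the spline of a SplinePathBP actor found in the level at BeginPlay.
; MoveObject plays a timeline with its rate set from TimeToCompleteInSeconds, using its track to interpolate distance over the spline's length.
; Each update sets the actor's transform from that distance, sampling location in world space but rotation in the spline's local space.
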(event Custom|Move%20Object
  (bind _spline_ref (Variables|Default|GetSpline%20REF))
  (bind _spline (Variables|/Game/SplinePathBP.SplinePathBP_C|GetSpline _spline_ref))
  (Components|Timeline|SetPlayRate (Variables|Default|GetMove%20Object%20T) (/ 1.0 (Variables|Default|GetTime%20To%20Complete%20%28In%20Seconds%29)))
  (bind _move_track (Timeline|Move%20Object%20T Play)
    (:Update
      (Transformation|SetActorTransform (Math|Transform|MakeTransform (Spline|GetLocationatDistanceAlongSpline _spline (Math|Float|Lerp 0.0 (Spline|GetSplineLength (Variables|/Game/SplinePathBP.SplinePathBP_C|GetSpline (Variables|Default|GetSpline%20REF))) _move_track) "World") (Spline|GetRotationatDistanceAlongSpline _spline (Math|Float|Lerp 0.0 (Spline|GetSplineLength (Variables|/Game/SplinePathBP.SplinePathBP_C|GetSpline (Variables|Default|GetSpline%20REF))) _move_track) "Local") "1.000000,1.000000,1.000000")))))

(event EventBeginPlay
  (bind _returnvalue (Actor|GetActorOfClass "/Game/SplinePathBP.SplinePathBP_C"))
  (Variables|Default|SetSpline%20REF _returnvalue)
  (CallFunction|MoveObject))

(fn ConstructionScript)